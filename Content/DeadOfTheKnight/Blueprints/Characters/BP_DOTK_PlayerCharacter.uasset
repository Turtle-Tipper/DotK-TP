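; Player character Blueprint for Dead of the Knight, wiring up the HUD, inventory window and item pickup.
; BeginPlay adds the character HUD to the viewport.
; The inventory action toggles the window, creating it or removing it and clearing its reference.
; The pickup action, gated by an overlap flag, passes the first overlapping DOTK_ItemBase to AddToInventory, which is defined outside these graphs.
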(event `InputAction|Open / Close Inventory`
  (params (Key :type "Key Structure"))
  ;[1 1 1] Action Binding for opening inventory window
  (:`Pressed`
    (bind _inventorymenuref (`self.InventoryMenuRef`)
      (:`then`
        (`Widget.RemoveFromParent` _inventorymenuref)
        (set `self.InventoryMenuRef` null))
      (:`else`
        (bind _returnvalue (`|CreateWidget` "/Game/DeadOfTheKnight/Blueprints/UI/WBP_InventoryWindow.WBP_InventoryWindow_C" (`GameplayStatics.GetPlayerController` 0)))
        (bind _output_get (set `self.InventoryMenuRef` _returnvalue))
        (`UserWidget.AddToViewport` _output_get 0)))))

(event `InputAction|Pick Up Item`
  (params (Key :type "Key Structure"))
  ;[1 1 1] Action binding for pick up item
  (:`Pressed`
    (if (`self.bIsOverlappingItem`)
      (bind _asdotk_item_base (cast `DOTK_ItemBase` (`|GetArrayItem` (`self.GetOverlappingActors` "/Script/DeadOfTheKnightTP.DOTK_ItemBase"))))
      (`self.AddToInventory` _asdotk_item_base))))

(event `self.ReceiveBeginPlay`
  ;[1 1 1] Create and Add Character HUD to viewport
  (bind _returnvalue (`|CreateWidget` "/Game/DeadOfTheKnight/Blueprints/UI/WBP_CharacterHUD.WBP_CharacterHUD_C"))
  (`UserWidget.AddToViewport` _returnvalue 0))

(fn `UserConstructionScript`)