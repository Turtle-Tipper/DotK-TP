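; Base weapon actor that the character picks up, holds in the right hand and uses to damage enemies.
; Attach destroys any current weapon and snaps this one to the hand socket, while remove destroys it and resets base attack speed.
; The interaction box toggles the player's item-overlap flag and pickup prompt, named through the empty SetCorrectItemName hook.
; Mesh overlaps damage enemies using the equipped weapon's damage, gated by HasAttacked and HasDealtDamage.
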(event `Remove Weapon`
  (params (`Character Reference` :type "DOTK_PlayerCharacter Object Reference"))
  ;[1 1 1] Remove weapon
  (bind _currentmainweapon (`DOTK_PlayerCharacter.CurrentMainWeapon` `Character Reference`)
    (:`then`
      (bind _asbp_weapon_base (cast `/Game/DeadOfTheKnight/Blueprints/GameObjects/Items/Equipment/Weapons/BP_WeaponBase` _currentmainweapon))
      (bind _itemmesh (`DOTK_ItemBase.ItemMesh` _asbp_weapon_base))
      (`PrimitiveComponent.SetCollisionEnabled` _itemmesh "NoCollision")
      (`SceneComponent.K2_DetachFromComponent` _itemmesh "KeepRelative" "KeepRelative" "KeepRelative" true)
      (set `DeadOfTheKnightTPCharacter.BaseAttackSpeed` 1.0 `Character Reference`)
      (`self.K2_DestroyActor` _currentmainweapon))
    (:`else`)))

(event `Attach Weapon`
  (params (`Character Reference` :type "/Game/DeadOfTheKnight/Blueprints/Characters/BP_DOTK_PlayerCharacter Object Reference"))
  ;[1 1 1] Weapon attachment
  (bind _currentmainweapon (`DOTK_PlayerCharacter.CurrentMainWeapon` `Character Reference`)
    (:`then`
      (bind _asbp_weapon_base (cast `/Game/DeadOfTheKnight/Blueprints/GameObjects/Items/Equipment/Weapons/BP_WeaponBase` _currentmainweapon))
      (bind _itemmesh (`DOTK_ItemBase.ItemMesh` _asbp_weapon_base))
      (`PrimitiveComponent.SetCollisionEnabled` _itemmesh "NoCollision")
      (`SceneComponent.K2_DetachFromComponent` _itemmesh "KeepRelative" "KeepRelative" "KeepRelative" true)
      (`self.K2_DestroyActor` _currentmainweapon))
    (:`else`
      _))
  (set `DOTK_PlayerCharacter.CurrentMainWeapon` self `Character Reference`)
  (`SceneComponent.K2_AttachToComponent` (`self.RootSceneComponent`) (`Character.Mesh` `Character Reference`) "socket_hand_r" "SnapToTarget" "SnapToTarget" "KeepRelative" true))

(event `self.InteractionBox.OnComponentBeginOverlap`
  (params (OverlappedComponent :type "PrimitiveComponent Object Reference") (OtherActor :type "Actor Object Reference") (OtherComp :type "PrimitiveComponent Object Reference") (OtherBodyIndex :type Integer) (bFromSweep :type Boolean) (SweepResult :type "HitResult Structure (by ref)"))
  ;[1 1 1] Create pick up item prompt widget
  (bind _asbp_dotk_player_character (cast `/Game/DeadOfTheKnight/Blueprints/Characters/BP_DOTK_PlayerCharacter` OtherActor))
  (set `DOTK_PlayerCharacter.bIsOverlappingItem` true _asbp_dotk_player_character)
  (bind _returnvalue (`|CreateWidget` "/Game/DeadOfTheKnight/Blueprints/UI/WBP_PickupItemPrompt.WBP_PickUpItemPrompt_C"))
  (`self.SetCorrectItemName` _returnvalue)
  (`UserWidget.AddToViewport` _returnvalue 0))

(event `self.InteractionBox.OnComponentEndOverlap`
  (params (OverlappedComponent :type "PrimitiveComponent Object Reference") (OtherActor :type "Actor Object Reference") (OtherComp :type "PrimitiveComponent Object Reference") (OtherBodyIndex :type Integer))
  ;[1 1 1] Remove all pick up item prompt widgets
  (bind _asbp_dotk_player_character (cast `/Game/DeadOfTheKnight/Blueprints/Characters/BP_DOTK_PlayerCharacter` OtherActor))
  (set `DOTK_PlayerCharacter.bIsOverlappingItem` false _asbp_dotk_player_character)
  (bind _foundwidgets (`WidgetBlueprintLibrary.GetAllWidgetsOfClass` "/Game/DeadOfTheKnight/Blueprints/UI/WBP_PickupItemPrompt.WBP_PickUpItemPrompt_C"))
  (for _array_element _foundwidgets
    (`Widget.RemoveFromParent` _array_element)))

(event `self.ItemMesh.OnComponentBeginOverlap`
  (params (OverlappedComponent :type "PrimitiveComponent Object Reference") (OtherActor :type "Actor Object Reference") (OtherComp :type "PrimitiveComponent Object Reference") (OtherBodyIndex :type Integer) (bFromSweep :type Boolean) (SweepResult :type "HitResult Structure (by ref)"))
  ;[1 1 1] Deal damage to EnemyCharacter if it is overlapped by ItemMesh while HasAttacked is true and HasDealtDamage is false.
  (bind _asbp_enemy_base (cast `/Game/DeadOfTheKnight/Blueprints/Characters/Enemies/BP_EnemyBase` OtherActor))
  (bind _asdead_of_the_knight_tpcharacter (cast `DeadOfTheKnightTPCharacter` (`GameplayStatics.GetPlayerCharacter` 0)))
  (bind _asbp_weapon_base (cast `/Game/DeadOfTheKnight/Blueprints/GameObjects/Items/Equipment/Weapons/BP_WeaponBase` (`DeadOfTheKnightTPCharacter.CurrentMainWeapon` _asdead_of_the_knight_tpcharacter)))
  (if (`DeadOfTheKnightTPCharacter.bHasAttacked` _asdead_of_the_knight_tpcharacter)
    (if (not (`DOTK_WeaponBase.bHasDealtDamage` _asbp_weapon_base))
      (`DotK_HealthComponent.TakeDamage` (`DeadOfTheKnightTPCharacter.HealthComponent` _asbp_enemy_base) (`DOTK_WeaponBase.BaseAttackDamage` _asbp_weapon_base))
      (set `self.bHasDealtDamage` true))))

(fn `SetCorrectItemName`
  (params (`Widget Ref` :type "/Game/DeadOfTheKnight/Blueprints/UI/WBP_PickupItemPrompt Object Reference")))

(fn `UserConstructionScript`)