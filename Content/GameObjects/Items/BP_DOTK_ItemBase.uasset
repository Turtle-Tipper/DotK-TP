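; BP_DOTK_ItemBase is an item base Blueprint that shows a pickup prompt when the player character overlaps it.
; On overlap begin it sets the player's IsOverlappingItem flag, creates WBP_PickupItemPrompt and passes it through SetCorrectItemName before display.
; On overlap end it clears the flag and removes every top-level prompt widget, not just its own.
; SetCorrectItemName is empty here, leaving the prompt's item name unset.
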(event `self.ReceiveActorBeginOverlap`
  (params (OtherActor :type "Actor Object Reference"))
  (bind _asbp_dotk_player_character (cast `/Game/Characters/BP_DOTK_PlayerCharacter` OtherActor))
  (set `DOTK_PlayerCharacter.bIsOverlappingItem` true _asbp_dotk_player_character)
  (bind _returnvalue (`|CreateWidget` "/Game/UI/WBP_PickupItemPrompt.WBP_PickupItemPrompt_C"))
  (`self.SetCorrectItemName` _returnvalue)
  (`UserWidget.AddToViewport` _returnvalue 0))

(event `self.ReceiveActorEndOverlap`
  (params (OtherActor :type "Actor Object Reference"))
  (bind _asbp_dotk_player_character (cast `/Game/Characters/BP_DOTK_PlayerCharacter` OtherActor))
  (set `DOTK_PlayerCharacter.bIsOverlappingItem` false _asbp_dotk_player_character)
  (bind _foundwidgets (`WidgetBlueprintLibrary.GetAllWidgetsOfClass` "/Game/UI/WBP_PickupItemPrompt.WBP_PickupItemPrompt_C"))
  (for _array_element _foundwidgets
    (`Widget.RemoveFromParent` _array_element)))

(fn `SetCorrectItemName`
  (params (`Widget Reference` :type "/Game/UI/WBP_PickupItemPrompt Object Reference")))

(fn `UserConstructionScript`)